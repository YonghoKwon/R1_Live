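; BP_R1Pawn is a pawn Blueprint that scaffolds Enhanced Input handling, with no working logic.
; BeginPlay, the IA_Test, IA_Move and IA_Turn events, and the construction script are all empty.
; Disconnected nodes would add and remove the IMC_Default mapping context, print debug text, and offset the pawn along world X by input, but none of them run.
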(event `self.ReceiveBeginPlay`)

(event `EnhancedInput|/Game/Input/IA_Test`
  (params (ActionValue :type Boolean) (ElapsedSeconds :type "Float (double-precision)") (TriggeredSeconds :type "Float (double-precision)") (InputAction :type "InputAction Object Reference" :default "/Game/Input/IA_Test.IA_Test")))

(event `EnhancedInput|/Game/Input/IA_Move`
  (params (ActionValue :type "Vector2D Structure") (ElapsedSeconds :type "Float (double-precision)") (TriggeredSeconds :type "Float (double-precision)") (InputAction :type "InputAction Object Reference" :default "/Game/Input/IA_Move.IA_Move")))

(event `EnhancedInput|/Game/Input/IA_Turn`
  (params (ActionValue :type "Vector2D Structure") (ElapsedSeconds :type "Float (double-precision)") (TriggeredSeconds :type "Float (double-precision)") (InputAction :type "InputAction Object Reference" :default "/Game/Input/IA_Turn.IA_Turn")))

(fn `UserConstructionScript`)