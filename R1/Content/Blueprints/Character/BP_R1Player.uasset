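; BP_R1Player is a player character Blueprint that currently holds only collision and trace debug experiments.
; Pressing 1 draws a visibility line trace from the camera to the point hit under the cursor, without using the result.
; Capsule hits print a test message.
; Three sphere trace variants at the TraceLocation component are left unconnected and never run.
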(event `Key|One`
  (params (Key :type "Key Structure")))

(event `Key|One`
  (params (Key :type "Key Structure"))
  (:`Pressed`
    (`KismetSystemLibrary.LineTraceSingle` :`Start` (`PlayerCameraManager.GetCameraLocation` (`GameplayStatics.GetPlayerCameraManager` 0)) :`End` (`.Location` (`GameplayStatics.BreakHitResult` (`PlayerController.GetHitResultUnderCursorByChannel` (`GameplayStatics.GetPlayerController` 0) "TraceTypeQuery1" true))) :`TraceChannel` "TraceTypeQuery1" :`DrawDebugType` "ForDuration")))

(event `self.CapsuleComponent.OnComponentHit`
  (params (HitComponent :type "PrimitiveComponent Object Reference") (OtherActor :type "Actor Object Reference") (OtherComp :type "PrimitiveComponent Object Reference") (NormalImpulse :type "Vector Structure") (Hit :type "HitResult Structure (by ref)"))
  (`KismetSystemLibrary.PrintString` "Hello"))

(fn `UserConstructionScript`)